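; Shooting game mode that gives access to pooled enemies and holds spawn logic for chase and wave enemies.
; BeginPlay caches the level's BP_EnemyPool, and getters fetch chase, wave, boss and bullet objects from its pools, with GetEnemy dispatching by type.
; Separate events spawn and activate enemies directly, bypassing the pool, switching from chase to wave after a count.
; The timer start and chase transform setup are disconnected.
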(event `self.ReceiveBeginPlay`
  (bind _outactors (`GameplayStatics.GetAllActorsOfClass` "/Game/ShootingGame/Blueprints/Enemy/BP_EnemyPool.BP_EnemyPool_C"))
  (set `self.EnemyPool` (`|GetArrayItem` _outactors)))

(event `SpawnEnemyChase`
  (for _array_element (`self.EnemyChaseTransform`)
    (bind _returnvalue (`|SpawnActorFromClass` "/Game/ShootingGame/Blueprints/Enemy/BP_EnemyChase.BP_EnemyChase_C" _array_element "AlwaysSpawn" "MultiplyWithRoot" null null))
    (bind _asbp_enemy_base (cast `/Game/ShootingGame/Blueprints/Enemy/BP_EnemyBase` _returnvalue))
    (`/Game/ShootingGame/Blueprints/ObjectPool/BP_PoolingObject.OnActivate` _asbp_enemy_base)
    (bind _result (`/Engine/EditorBlueprintResources/StandardMacros.IncrementInt` (`self.ChaseCount`))
      (:`  `
        (if (>= _result (`self.ChaseEndCount`))
          (`KismetSystemLibrary.K2_ClearAndInvalidateTimerHandle` (`self.ChaseTimer`))
          (`KismetSystemLibrary.Delay` 2.0)
          (`self.SpawnEnemyWave`))))))

(event `SpawnEnemyWave`
  (for _array_element (`self.EnemyWaveTransform`)
    (bind _returnvalue (`|SpawnActorFromClass` "/Game/ShootingGame/Blueprints/Enemy/BP_EnemyWave.BP_EnemyWave_C" _array_element "AlwaysSpawn" "MultiplyWithRoot" null null))
    (bind _asbp_enemy_base (cast `/Game/ShootingGame/Blueprints/Enemy/BP_EnemyBase` _returnvalue))
    (`/Game/ShootingGame/Blueprints/ObjectPool/BP_PoolingObject.OnActivate` _asbp_enemy_base)))

(fn `GetEnemy`
  (params (Type :type "/Game/ShootingGame/Blueprints/Enemy/E_EnemyType Enum" :default "NewEnumerator0") (SpawnTransform :type "Transform Structure"))
  (returns (NewEnemy :type "/Game/ShootingGame/Blueprints/Enemy/BP_EnemyBase Object Reference"))
  (switch `/Game/ShootingGame/Blueprints/Enemy/E_EnemyType` Type
    (:`NewEnumerator0`
      (bind _newenemy (`self.GetEnemyChase` SpawnTransform))
      (return _newenemy))
    (:`NewEnumerator1`
      (bind _newenemy_2 (`self.GetEnemyWave` SpawnTransform))
      (return _newenemy_2))
    (:`NewEnumerator2`
      (bind _newenemy_3 (`self.GetEnemyBoss` SpawnTransform))
      (return _newenemy_3))))

(fn `GetEnemyBoss`
  (params (SpawnTransform :type "Transform Structure"))
  (returns (NewEnemy :type "/Game/ShootingGame/Blueprints/Enemy/BP_EnemyBase Object Reference"))
  (bind _enemypool (`self.EnemyPool`))
  (`/Engine/EditorBlueprintResources/StandardMacros.IsValid` _enemypool
    (:`Is Valid`
      (bind _newobject (`/Game/ShootingGame/Blueprints/ObjectPool/AC_ObjectPool.GetObject` (`/Game/ShootingGame/Blueprints/Enemy/BP_EnemyPool.Pool_Boss` _enemypool) SpawnTransform))
      (bind _asbp_enemy_base (cast `/Game/ShootingGame/Blueprints/Enemy/BP_EnemyBase` _newobject))
      (return _asbp_enemy_base))))

(fn `GetEnemyChase`
  (params (SpawnTransform :type "Transform Structure"))
  (returns (NewEnemy :type "/Game/ShootingGame/Blueprints/Enemy/BP_EnemyBase Object Reference"))
  (bind _enemypool (`self.EnemyPool`))
  (`/Engine/EditorBlueprintResources/StandardMacros.IsValid` _enemypool
    (:`Is Valid`
      (bind _newobject (`/Game/ShootingGame/Blueprints/ObjectPool/AC_ObjectPool.GetObject` (`/Game/ShootingGame/Blueprints/Enemy/BP_EnemyPool.Pool_Chase` _enemypool) SpawnTransform))
      (bind _asbp_enemy_base (cast `/Game/ShootingGame/Blueprints/Enemy/BP_EnemyBase` _newobject))
      (return _asbp_enemy_base))))

(fn `GetEnemyChaseBullet`
  (params (SpawnTransform :type "Transform Structure"))
  (returns (NewEnemy :type "/Game/ShootingGame/Blueprints/Enemy/BP_EnemyBase Object Reference"))
  (bind _enemypool (`self.EnemyPool`))
  (`/Engine/EditorBlueprintResources/StandardMacros.IsValid` _enemypool
    (:`Is Valid`
      (bind _newobject (`/Game/ShootingGame/Blueprints/ObjectPool/AC_ObjectPool.GetObject` (`/Game/ShootingGame/Blueprints/Enemy/BP_EnemyPool.Pool_ChaseBullet` _enemypool) SpawnTransform))
      (bind _asbp_enemy_base (cast `/Game/ShootingGame/Blueprints/Enemy/BP_EnemyBase` _newobject))
      (return _asbp_enemy_base))))

(fn `GetEnemyWave`
  (params (SpawnTransform :type "Transform Structure"))
  (returns (NewEnemy :type "/Game/ShootingGame/Blueprints/Enemy/BP_EnemyBase Object Reference"))
  (bind _enemypool (`self.EnemyPool`))
  (`/Engine/EditorBlueprintResources/StandardMacros.IsValid` _enemypool
    (:`Is Valid`
      (bind _newobject (`/Game/ShootingGame/Blueprints/ObjectPool/AC_ObjectPool.GetObject` (`/Game/ShootingGame/Blueprints/Enemy/BP_EnemyPool.Pool_Wave` _enemypool) SpawnTransform))
      (bind _asbp_enemy_base (cast `/Game/ShootingGame/Blueprints/Enemy/BP_EnemyBase` _newobject))
      (return _asbp_enemy_base))))

(fn `GetEnemyWaveBullet`
  (params (SpawnTransform :type "Transform Structure"))
  (returns (NewEnemy :type "/Game/ShootingGame/Blueprints/Enemy/BP_EnemyBase Object Reference"))
  (bind _enemypool (`self.EnemyPool`))
  (`/Engine/EditorBlueprintResources/StandardMacros.IsValid` _enemypool
    (:`Is Valid`
      (bind _newobject (`/Game/ShootingGame/Blueprints/ObjectPool/AC_ObjectPool.GetObject` (`/Game/ShootingGame/Blueprints/Enemy/BP_EnemyPool.Pool_WaveBullet` _enemypool) SpawnTransform))
      (bind _asbp_enemy_base (cast `/Game/ShootingGame/Blueprints/Enemy/BP_EnemyBase` _newobject))
      (return _asbp_enemy_base))))

(fn `UserConstructionScript`)