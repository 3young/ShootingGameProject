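; HUD for the shooting game that puts the main UI widget on screen and hooks it to gameplay events.
; On BeginPlay it creates WBP_UI for the first player, stores it and adds it to the viewport.
; It then binds delegates to score updates from GS_ShootingGame and the death event of the BP_PlayerFlightUsePool pawn, stopping if either cast fails.
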(event `self.ReceiveBeginPlay`
  (bind _returnvalue (`|CreateWidget` "/Game/ShootingGame/UI/WBP_UI.WBP_UI_C" (`GameplayStatics.GetPlayerController` 0)))
  (bind _output_get (set `self.UI Widget` _returnvalue))
  (`UserWidget.AddToViewport` _output_get 0)
  (bind _asgs_shooting_game (cast `/Game/ShootingGame/Blueprints/Frameworks/GS_ShootingGame` (`GameplayStatics.GetGameState`)))
  (add `/Game/ShootingGame/Blueprints/Frameworks/GS_ShootingGame.ScoreUpdated` _asgs_shooting_game (`|CreateDelegate` _output_get :!event `RefreshScore`))
  (bind _asbp_player_flight_use_pool (cast `/Game/ShootingGame/Blueprints/Player/BP_PlayerFlightUsePool` (`GameplayStatics.GetPlayerPawn` 0)))
  (add `/Game/ShootingGame/Blueprints/Player/BP_PlayerFlightUsePool.OnDie` _asbp_player_flight_use_pool (`|CreateDelegate` _output_get :!event `ShowGameOverPanel`)))

(fn `UserConstructionScript`)