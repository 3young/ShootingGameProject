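; BP_Shot is a physics-driven projectile Blueprint for a shooting game.
; When the IA_Attack input completes, its own event graph spawns a new BP_Shot at the player pawn's location and calls OnShooted on it.
; OnShooted applies a large impulse to the Shot component, computed from the pawn's forward vector plus a constant offset, then scaled.
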(event `EnhancedInput|/Game/ShootingGame/Input/IA_Attack`
  (params (ActionValue :type Boolean) (ElapsedSeconds :type "Float (double-precision)") (TriggeredSeconds :type "Float (double-precision)") (InputAction :type "InputAction Object Reference" :default "/Game/ShootingGame/Input/IA_Attack.IA_Attack"))
  (:`Completed`
    (bind _returnvalue (`|SpawnActorFromClass` "BP_Shot_C" (`KismetMathLibrary.MakeTransform` (`self.K2_GetActorLocation` (`GameplayStatics.GetPlayerPawn` 0))) "Undefined" "MultiplyWithRoot" null null))
    (`self.OnShooted` _returnvalue)))

(fn `OnShooted`
  (`PrimitiveComponent.AddImpulse` (`self.Shot`) (* (+ (`self.GetActorForwardVector` (`GameplayStatics.GetPlayerPawn` 0)) 10.0) 10000) "None" false))

(fn `UserConstructionScript`)