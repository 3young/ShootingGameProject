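; Pooled projectile that flies forward and turns into a timed damage area when it overlaps an actor not tagged Player or Bullet.
; Activate and deactivate events toggle collision, effects and movement for reuse, with a lifetime timer set on launch.
; The area tracks overlapping actors for a looping damage timer, though DamageAll returns after the first one, then deactivates.
; The construction script tints both effects.
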(event `self.ReceiveActorBeginOverlap`
  (params (OtherActor :type "Actor Object Reference"))
  (if (not (or (`self.ActorHasTag` OtherActor "Player") (`self.ActorHasTag` OtherActor "Bullet")))
    (`self.SecondExplosion`)))

(event `self.Activate`
  (`parent.Activate`))

(event `self.Deactivate`
  (`parent.Deactivate`))

(event `self.OnActivate`
  (`PrimitiveComponent.SetCollisionEnabled` (`self.AreaCollision`) "NoCollision")
  (`ActorComponent.Deactivate` (`self.VFX_Area`))
  (`PrimitiveComponent.SetCollisionEnabled` (`self.ProjectileCollision`) "QueryOnly")
  (`ActorComponent.Activate` (`self.VFX_Projectile`) true)
  (`ActorComponent.Activate` (`self.ProjectileMovement`) true)
  (`ProjectileMovementComponent.SetVelocityInLocalSpace` (`self.ProjectileMovement`) (* (`KismetMathLibrary.Vector_Forward`) (`self.InitialSpeed`)))
  (`KismetSystemLibrary.K2_SetTimerDelegate` (`|CreateDelegate` :!event `SecondExplosion`) (`self.LifeTime`)))

(event `self.OnDeactivate`
  (`PrimitiveComponent.SetCollisionEnabled` (`self.AreaCollision`) "NoCollision")
  (`ActorComponent.Deactivate` (`self.VFX_Area`))
  (`PrimitiveComponent.SetCollisionEnabled` (`self.ProjectileCollision`) "NoCollision")
  (`ActorComponent.Deactivate` (`self.VFX_Projectile`))
  (`ActorComponent.Deactivate` (`self.ProjectileMovement`)))

(event `SecondExplosion`
  (`PrimitiveComponent.SetCollisionEnabled` (`self.AreaCollision`) "QueryOnly")
  (`ActorComponent.Activate` (`self.VFX_Area`) true)
  (`PrimitiveComponent.SetCollisionEnabled` (`self.ProjectileCollision`) "NoCollision")
  (`ActorComponent.Deactivate` (`self.VFX_Projectile`))
  (`ActorComponent.Deactivate` (`self.ProjectileMovement`))
  (bind _returnvalue (`KismetSystemLibrary.K2_SetTimerDelegate` (delegate `DamageToTarget`) 0.1 true))
  (`KismetSystemLibrary.Delay` (`self.SecondDuration`))
  (`KismetSystemLibrary.K2_ClearAndInvalidateTimerHandle` _returnvalue)
  (`self.Deactivate`))

(event `DamageToTarget`
  (`self.DamageAll`))

(event `self.AreaCollision.OnComponentBeginOverlap`
  (params (OverlappedComponent :type "PrimitiveComponent Object Reference") (OtherActor :type "Actor Object Reference") (OtherComp :type "PrimitiveComponent Object Reference") (OtherBodyIndex :type Integer) (bFromSweep :type Boolean) (SweepResult :type "HitResult Structure (by ref)"))
  (if (not (or (`self.ActorHasTag` OtherActor "Player") (`self.ActorHasTag` OtherActor "Bullet")))
    (`KismetArrayLibrary.Array_AddUnique` (`self.DamageTarget`) OtherActor)))

(event `self.AreaCollision.OnComponentEndOverlap`
  (params (OverlappedComponent :type "PrimitiveComponent Object Reference") (OtherActor :type "Actor Object Reference") (OtherComp :type "PrimitiveComponent Object Reference") (OtherBodyIndex :type Integer))
  (`KismetArrayLibrary.Array_RemoveItem` (`self.DamageTarget`) OtherActor))

(fn `UserConstructionScript`
  (`FXSystemComponent.SetVectorParameter` (`self.VFX_Projectile`) "ProjectileColor" (`KismetMathLibrary.Conv_LinearColorToVector` (`self.EffectColor`)))
  (`FXSystemComponent.SetVectorParameter` (`self.VFX_Area`) "BaseColor" (`KismetMathLibrary.Conv_LinearColorToVector` (`self.EffectColor`))))