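; Projectile actor for a shooting game that damages what it overlaps and expires after a set lifetime.
; A timer started on BeginPlay triggers the Destroy event, which spawns a pooled explosion effect at the projectile's location and removes it.
; Overlapping an actor without the Player or Bullet tag applies damage and destroys the projectile immediately, without spawning the explosion.
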(event `self.ReceiveBeginPlay`
  (`KismetSystemLibrary.K2_SetTimerDelegate` (delegate `Destroy`) (`self.LifeTime`)))

(event `Destroy`
  (`NiagaraFunctionLibrary.SpawnSystemAtLocation` (`self.ExplosionEffect`) (`self.K2_GetActorLocation`) (struct) (1.0 1.0 1.0) true true "AutoRelease")
  (`self.K2_DestroyActor`))

(event `self.ReceiveActorBeginOverlap`
  (params (OtherActor :type "Actor Object Reference"))
  (if (not (or (`self.ActorHasTag` OtherActor "Player") (`self.ActorHasTag` OtherActor "Bullet")))
    (`GameplayStatics.ApplyDamage` OtherActor (`self.Damage`))
    (`self.K2_DestroyActor`)))

(fn `UserConstructionScript`)