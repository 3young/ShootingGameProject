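; BP_EnemyFirstAttack is an enemy attack projectile that damages the player on overlap.
; BeginPlay starts a LifeTime timer bound to a custom Destroy event.
; Overlapping an actor tagged Player applies BaseDamage and calls the same Destroy event early.
; Destroy spawns the VFX_EnemyFirst effect at the projectile's location before removing the actor.
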(event `self.ReceiveBeginPlay`
  (`KismetSystemLibrary.K2_SetTimerDelegate` (delegate `Destroy`) (`self.LifeTime`)))

(event `Destroy`
  (`NiagaraFunctionLibrary.SpawnSystemAtLocation` "/Game/ShootingGame/Blueprints/Effect/VFX_EnemyFirst.VFX_EnemyFirst" (`self.K2_GetActorLocation`))
  (`self.K2_DestroyActor`))

(event `self.ReceiveActorBeginOverlap`
  (params (OtherActor :type "Actor Object Reference"))
  (if (`self.ActorHasTag` OtherActor "Player")
    (`GameplayStatics.ApplyDamage` null (`self.BaseDamage`))
    (`self.Destroy`)))

(fn `UserConstructionScript`)