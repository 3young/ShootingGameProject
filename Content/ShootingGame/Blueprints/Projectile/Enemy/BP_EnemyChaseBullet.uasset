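; Enemy projectile that, on activation, launches toward the player pawn's current location at MoveSpeed; the graph does not re-aim afterward.
; Overlapping a Player-tagged actor applies damage and deactivates the bullet.
; Activation and deactivation toggle velocity, mesh visibility and collision instead of spawning or destroying the actor.
; Deactivation spawns a pooled explosion, except on its first call, which only stops movement and sets IsInitialized.
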(event `self.OnActivate`
  (bind _staticmesh (`self.StaticMesh`))
  (set `MovementComponent.Velocity` (* (`KismetMathLibrary.Normal` (- (`self.K2_GetActorLocation` (`GameplayStatics.GetPlayerPawn` 0)) (`self.K2_GetActorLocation`))) (`self.MoveSpeed`)) (`self.ProjectileMovement`))
  (`PrimitiveComponent.SetCollisionEnabled` _staticmesh "QueryOnly")
  (`SceneComponent.SetVisibility` _staticmesh true false))

(event `self.OnDeactivate`
  (bind _staticmesh (`self.StaticMesh`))
  (set `MovementComponent.Velocity` (0.0 0.0 0.0) (`self.ProjectileMovement`))
  (if (`self.IsInitialized`)
    (`NiagaraFunctionLibrary.SpawnSystemAtLocation` (`self.SelfExplosion`) (`self.K2_GetActorLocation`) (struct) (1.0 1.0 1.0) true true "AutoRelease")
    (`SceneComponent.SetVisibility` _staticmesh false false)
    (`PrimitiveComponent.SetCollisionEnabled` _staticmesh "NoCollision")
    (else
      (set `self.IsInitialized` true))))

(event `self.ReceiveActorBeginOverlap`
  (params (OtherActor :type "Actor Object Reference"))
  (if (`self.ActorHasTag` OtherActor "Player")
    (`GameplayStatics.ApplyDamage` OtherActor (`self.BaseDamage`))
    (`self.Deactivate`)))

(fn `UserConstructionScript`)