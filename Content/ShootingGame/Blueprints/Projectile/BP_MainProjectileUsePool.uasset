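; BP_MainProjectileUsePool is a pooled projectile for the shooting game that is reused through Activate and Deactivate events.
; On activation it enables sphere query collision, starts Niagara and projectile movement along local forward, and sets a lifetime timer.
; Overlapping an actor not tagged Player or Bullet applies damage, spawns an auto-released explosion effect and deactivates the projectile.
; Deactivation switches off collision, Niagara and movement.
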(event `self.ReceiveActorBeginOverlap`
  (params (OtherActor :type "Actor Object Reference"))
  (if (not (or (`self.ActorHasTag` OtherActor "Player") (`self.ActorHasTag` OtherActor "Bullet")))
    (`GameplayStatics.ApplyDamage` OtherActor (`self.Base Damage`))
    (`NiagaraFunctionLibrary.SpawnSystemAtLocation` (`self.ExplosionEffect`) (`self.K2_GetActorLocation`) (struct) (1.0 1.0 1.0) true true "AutoRelease")
    (`self.Deactivate`)))

(event `/Game/ShootingGame/Blueprints/ObjectPool/BPI_PoolObject.Activate`
  (`parent.Activate`))

(event `/Game/ShootingGame/Blueprints/ObjectPool/BPI_PoolObject.Deactivate`
  (`parent.Deactivate`))

(event `self.OnActivate`
  (`PrimitiveComponent.SetCollisionEnabled` (`self.Sphere`) "QueryOnly")
  (`ActorComponent.Activate` (`self.Niagara`) true)
  (`ActorComponent.Activate` (`self.ProjectileMovement`) true)
  (`ProjectileMovementComponent.SetVelocityInLocalSpace` (`self.ProjectileMovement`) (* (`KismetMathLibrary.Vector_Forward`) (`self.MainInitialSpeed`)))
  (`KismetSystemLibrary.K2_SetTimerDelegate` (`|CreateDelegate` :!event `Deactivate`) (`self.LifeTime`)))

(event `self.OnDeactivate`
  (`PrimitiveComponent.SetCollisionEnabled` (`self.Sphere`) "NoCollision")
  (`ActorComponent.Deactivate` (`self.Niagara`))
  (`ActorComponent.Deactivate` (`self.ProjectileMovement`)))

(fn `UserConstructionScript`)