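; BP_PoolingEnemyObject is a pooled enemy object, judging by its name, that toggles between active and pooled states.
; Activate, when IsActivate is false, detaches the actor keeping world transform, calls the empty OnActivate hook and sets the flag.
; Deactivate calls the empty OnDeactivate hook, fires OnMainObjectReturnToPool with itself and clears the flag.
; As wired, Deactivate runs that sequence only when IsActivate is already false, so an active object skips it.
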(event `/Game/ShootingGame/Blueprints/ObjectPool/BPI_PoolObject.Activate`
  (if (== (`self.IsActivate`) false)
    (`self.K2_DetachFromActor` "KeepWorld" "KeepWorld" "KeepWorld")
    (`self.OnActivate`)
    (set `self.IsActivate` true)))

(event `/Game/ShootingGame/Blueprints/ObjectPool/BPI_PoolObject.Deactivate`
  (if (not (== (`self.IsActivate`) true))
    (`self.OnDeactivate`)
    (`self.OnMainObjectReturnToPool` self)
    (set `self.IsActivate` false)))

(event `OnActivate`)

(event `OnDeactivate`)

(fn `UserConstructionScript`)