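; Actor component that pools instances of a MainObject class for reuse in the shooting game.
; On BeginPlay it pre-spawns MainPoolSize deactivated actors, attaches them to its owner at an offset and binds each one's return-to-pool event.
; GetMainObject removes the first pooled actor, moves it to the requested transform and activates it.
; An empty pool grows by spawning another actor and retrying recursively.
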(event `self.ReceiveBeginPlay`
  (`KismetArrayLibrary.Array_Clear` (`self.MainPool`))
  (for _ (range (`self.MainPoolSize`))
    (`self.SpawnMainObjectToPool`)))

(event `SpawnMainObjectToPool`
  (bind _returnvalue (`|SpawnActorFromClass` (`self.MainObject`) (`KismetMathLibrary.MakeTransform` (0.0 0.0 0.0)) "AlwaysSpawn" "MultiplyWithRoot" (`self.GetOwner`) null))
  (`/Game/ShootingGame/Blueprints/ObjectPool/BP_PoolingMainObject.OnDeactivate` _returnvalue)
  (`self.MoveToMainPoolChild` _returnvalue)
  (add `/Game/ShootingGame/Blueprints/ObjectPool/BP_PoolingMainObject.OnMainObjectReturnToPool` _returnvalue (`|CreateDelegate` :!event `MoveToMainPoolChild`)))

(event `MoveToMainPoolChild`
  (params (ToMainPool :type "/Game/ShootingGame/Blueprints/ObjectPool/BP_PoolingMainObject Object Reference"))
  (`Actor.K2_AttachToActor` ToMainPool (`self.GetOwner`) "None" "SnapToTarget" "SnapToTarget" "SnapToTarget" true)
  (`Actor.K2_SetActorRelativeLocation` ToMainPool (`self.Offset`) false false)
  (`KismetArrayLibrary.Array_Add` (`self.MainPool`) ToMainPool))

(fn `GetMainObject`
  (params (SpawnTransform :type "Transform Structure (by ref)"))
  (returns (NewMainObject :type "/Game/ShootingGame/Blueprints/ObjectPool/BP_PoolingMainObject Object Reference"))
  (locals (Result :type "/Game/ShootingGame/Blueprints/ObjectPool/BP_PoolingMainObject Object Reference"))
  (bind _result (`local.Result`))
  (if (> (`KismetArrayLibrary.Array_Length` (`self.MainPool`)) 0)
    (bind _output_get (set `local.Result` (`|GetArrayItem` (`self.MainPool`))))
    (`KismetArrayLibrary.Array_RemoveItem` (`self.MainPool`) _output_get)
    (`Actor.K2_SetActorTransform` _output_get SpawnTransform false false)
    (`/Game/ShootingGame/Blueprints/ObjectPool/BP_PoolingMainObject.Activate` _result)
    (return _result)
    (else
      (`self.SpawnMainObjectToPool`)
      (bind _newmainobject (`self.GetMainObject` SpawnTransform))
      (return _newmainobject))))