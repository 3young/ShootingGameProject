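; Actor component that pools enemy actors for the shooting game, pre-spawning deactivated instances on BeginPlay.
; GetEnemyObject removes the first pooled enemy, places and activates it, or spawns another and retries recursively when empty.
; Each spawn binds a return-to-pool event and calls MoveToEnemyPoolChild, whose attach-to-owner and add-to-pool nodes are disconnected, so nothing here refills the pool.
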(event `self.ReceiveBeginPlay`
  (`KismetArrayLibrary.Array_Clear` (`self.EnemyPool`))
  (for _ (range (`self.EnemyPoolSize`))
    (`self.SpawnEnemyObjectToPool`)))

(event `SpawnEnemyObjectToPool`
  (bind _returnvalue (`|SpawnActorFromClass` (`self.EnemyObject`) (`KismetMathLibrary.MakeTransform` (0.0 0.0 0.0)) "AlwaysSpawn" "MultiplyWithRoot" (`self.GetOwner`) null))
  (`/Game/ShootingGame/Blueprints/ObjectPool/BP_PoolingEnemyObject.OnDeactivate` _returnvalue)
  (`self.MoveToEnemyPoolChild` _returnvalue)
  (add `/Game/ShootingGame/Blueprints/ObjectPool/BP_PoolingEnemyObject.OnMainObjectReturnToPool` _returnvalue (`|CreateDelegate` :!event `MoveToEnemyPoolChild`)))

(event `MoveToEnemyPoolChild`
  (params (ToMainPool :type "/Game/ShootingGame/Blueprints/ObjectPool/BP_PoolingEnemyObject Object Reference")))

(fn `GetEnemyObject`
  (params (SpawnTransform :type "Transform Structure (by ref)"))
  (returns (NewMainObject :type "/Game/ShootingGame/Blueprints/ObjectPool/BP_PoolingEnemyObject Object Reference"))
  (locals (Result :type "/Game/ShootingGame/Blueprints/ObjectPool/BP_PoolingEnemyObject Object Reference"))
  (bind _result (`local.Result`))
  (if (> (`KismetArrayLibrary.Array_Length` (`self.EnemyPool`)) 0)
    (bind _output_get (set `local.Result` (`|GetArrayItem` (`self.EnemyPool`))))
    (`KismetArrayLibrary.Array_RemoveItem` (`self.EnemyPool`) _output_get)
    (`Actor.K2_SetActorTransform` _output_get SpawnTransform false false)
    (`/Game/ShootingGame/Blueprints/ObjectPool/BP_PoolingEnemyObject.Activate` _result)
    (return _result)
    (else
      (`self.SpawnEnemyObjectToPool`)
      (bind _newmainobject (`self.GetEnemyObject` SpawnTransform))
      (return _newmainobject))))