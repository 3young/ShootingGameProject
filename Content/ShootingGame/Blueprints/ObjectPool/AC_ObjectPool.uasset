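; Actor component that keeps a reusable pool of BaseObject actors for its owner.
; BeginPlay pre-spawns PoolSize deactivated actors, attaches each to the owner at an offset and binds to its return-to-pool event.
; GetObject takes the first pooled actor, moves it to the requested transform and activates it.
; An empty pool grows on demand by spawning another actor and retrying recursively.
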(event `self.ReceiveBeginPlay`
  (`KismetArrayLibrary.Array_Clear` (`self.Pool`))
  (for _ (range (`self.PoolSize`))
    (`self.SpawnObjectToPool`)))

(event `SpawnObjectToPool`
  (bind _returnvalue (`|SpawnActorFromClass` (`self.BaseObject`) (`KismetMathLibrary.MakeTransform` (0.0 0.0 0.0)) "AlwaysSpawn" "MultiplyWithRoot" (`self.GetOwner`) null))
  (`/Game/ShootingGame/Blueprints/ObjectPool/BP_PoolingObject.Deactivate` _returnvalue)
  (`self.MoveToPoolChild` _returnvalue)
  (add `/Game/ShootingGame/Blueprints/ObjectPool/BP_PoolingObject.OnObjectReturnToPool` _returnvalue (`|CreateDelegate` :!event `MoveToPoolChild`)))

(event `MoveToPoolChild`
  (params (ToPool :type "/Game/ShootingGame/Blueprints/ObjectPool/BP_PoolingObject Object Reference"))
  (`Actor.K2_AttachToActor` ToPool (`self.GetOwner`) "None" "SnapToTarget" "SnapToTarget" "SnapToTarget" true)
  (`Actor.K2_SetActorRelativeLocation` ToPool (`self.Offset`) false false)
  (`KismetArrayLibrary.Array_Add` (`self.Pool`) ToPool))

(fn `GetObject`
  (params (SpawnTransform :type "Transform Structure (by ref)"))
  (returns (NewObject :type "/Game/ShootingGame/Blueprints/ObjectPool/BP_PoolingObject Object Reference"))
  (locals (Result :type "/Game/ShootingGame/Blueprints/ObjectPool/BP_PoolingObject Object Reference"))
  (bind _result (`local.Result`))
  (if (> (`KismetArrayLibrary.Array_Length` (`self.Pool`)) 0)
    (bind _output_get (set `local.Result` (`|GetArrayItem` (`self.Pool`))))
    (`KismetArrayLibrary.Array_RemoveItem` (`self.Pool`) _output_get)
    (`Actor.K2_SetActorTransform` _output_get SpawnTransform false false)
    (`/Game/ShootingGame/Blueprints/ObjectPool/BP_PoolingObject.Activate` _result)
    (return _result)
    (else
      (`self.SpawnObjectToPool`)
      (bind _newobject (`self.GetObject` SpawnTransform))
      (return _newobject))))