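; Projectile pool actor for the shooting game that pre-spawns BP_Projectile actors at BeginPlay.
; InitializePool spawns hidden projectiles at the pool's root transform, stores them in BulletPool and sets a single shared IsHidden flag.
; GetPooledBullet, also run at BeginPlay, copies every pooled bullet into AvailableBullet while that flag is true, printing each index, and returns none.
; ReturnPooledBullet only hides the pool actor itself.
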(event `self.ReceiveBeginPlay`
  (`self.InitializePool`)
  (`self.GetPooledBullet`))

(fn `GetPooledBullet`
  (for _array_element (`self.BulletPool`)
    (if (`self.IsHidden`)
      (bind _returnvalue (`KismetArrayLibrary.Array_Add` (`self.AvailableBullet `) _array_element))
      (`KismetSystemLibrary.PrintString` (`KismetStringLibrary.Conv_IntToString` _returnvalue)))))

(fn `InitializePool`
  (for _ (range (+ (`self.InitialPoolSize`) 1))
    (bind _returnvalue (`|SpawnActorFromClass` "/Game/ShootingGame/Blueprints/BP_Projectile.BP_Projectile_C" (`SceneComponent.K2_GetComponentToWorld` (`self.DefaultSceneRoot`)) "Undefined" "MultiplyWithRoot" null null))
    (`self.SetActorHiddenInGame` _returnvalue true)
    (`KismetArrayLibrary.Array_Add` (`self.BulletPool`) _returnvalue)
    (set `self.IsHidden` true)))

(fn `ReturnPooledBullet`
  (`self.SetActorHiddenInGame` true))

(fn `UserConstructionScript`)