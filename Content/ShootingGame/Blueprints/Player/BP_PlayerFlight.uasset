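; Player-controlled ship for the shooting game, moving on the XY plane through Enhanced Input.
; Each fire press spawns an actor, alternating between two muzzle sockets via a toggle flag.
; Every tick, crossing an X or Y border teleports the ship to OtherSideLocation, whose negated-XY vector appears unconnected.
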(event `self.ReceiveBeginPlay`
  (`EnhancedInputSubsystemInterface.AddMappingContext` (pcsubsystem `EnhancedInputLocalPlayerSubsystem` (`GameplayStatics.GetPlayerController` 0)) "/Game/ShootingGame/Input/IMC_PlayerFlight.IMC_PlayerFlight" 0 (struct)))

(event `self.ReceiveTick`
  (params (DeltaSeconds :type "Float (single-precision)"))
  (`self.WarpToOtherSide`))

(event `EnhancedInput|/Game/ShootingGame/Input/IA_Move`
  (params (ActionValue :type "Vector2D Structure") (ElapsedSeconds :type "Float (double-precision)") (TriggeredSeconds :type "Float (double-precision)") (InputAction :type "InputAction Object Reference" :default "/Game/ShootingGame/Input/IA_Move.IA_Move"))
  (bind (_returnvalue_x _returnvalue_y) (`KismetMathLibrary.BreakVector2D` (`KismetMathLibrary.Normal2D` ActionValue)))
  (:`Triggered`
    (`self.AddMovementInput` (`KismetMathLibrary.MakeVector` _returnvalue_y _returnvalue_x))))

(event `EnhancedInput|/Game/ShootingGame/Input/IA_Fire`
  (params (ActionValue :type Boolean) (ElapsedSeconds :type "Float (double-precision)") (TriggeredSeconds :type "Float (double-precision)") (InputAction :type "InputAction Object Reference" :default "/Game/ShootingGame/Input/IA_Fire.IA_Fire"))
  (:`Started`
    (`self.Fire`)))

(event `Fire`
  (bind _firetransform (`self.GetFireTransform`))
  (`|SpawnActorFromClass` (`self.Class`) _firetransform "Undefined" "MultiplyWithRoot" null null))

(fn `GetFireTransform`
  (returns (FireTransform :type "Transform Structure"))
  (bind _playerflight (`self.PlayerFlight`))
  (if (`self.FireLocationSelector`)
    (set `self.FireLocationSelector` false)
    (return (`SceneComponent.GetSocketTransform` _playerflight "FireSocket1" "RTS_World"))
    (else
      (set `self.FireLocationSelector` true)
      (return (`SceneComponent.GetSocketTransform` _playerflight "FireSocket2" "RTS_World")))))

(fn `UserConstructionScript`)

(fn `WarpToOtherSide`
  (locals (BorderY :type Integer :default 3500) (BorderX :type Integer :default 2000))
  (bind (_returnvalue_x _returnvalue_y) (`KismetMathLibrary.BreakVector` (`self.K2_GetActorLocation`)))
  (bind _returnvalue_x_2 (`KismetMathLibrary.BreakVector` (`self.K2_GetActorLocation`)))
  (`|ExecutionSequence`
    (:`then_0`
      (if (> _returnvalue_x_2 (`local.BorderX`))
        (`self.K2_SetActorLocation` (`self.OtherSideLocation`) false true :!label _label)
        (elif (< _returnvalue_x_2 (* (`local.BorderX`) -1))
          (goto _label))))
    (:`then_1`
      (if (> _returnvalue_y (`local.BorderY`))
        (`self.K2_SetActorLocation` (`self.OtherSideLocation`) false true :!label _label_2)
        (elif (< _returnvalue_y (* (`local.BorderY`) -1))
          (goto _label_2))))))