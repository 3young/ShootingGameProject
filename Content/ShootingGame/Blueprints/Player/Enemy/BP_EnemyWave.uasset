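; BP_EnemyWave is a shooting-game enemy whose mesh sways sideways while it fires chase bullets in bursts.
; On activation, a timeline drives the mesh's relative offset along the left axis, scaled by Width.
; FireProcess starts a looping timer that requests bullets from the GameMode at AttackSocket until the repeat count is reached.
; Nothing here triggers FireProcess: its only call is unwired, and the post-burst delay leads nowhere.
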(event `/Game/ShootingGame/Blueprints/ObjectPool/BP_PoolingObject.OnActivate`
  (`parent.OnActivate`)
  (bind (_direction _wavealpha) (`Timeline|TL_Wave` :!via `PlayFromStart`)
    (:`Update`
      (`SceneComponent.K2_SetRelativeLocation` (`self.StaticMesh`) (* _wavealpha (`self.Width`) (`KismetMathLibrary.Vector_Left`)) false false))))

(event `FireProcess`
  (set `self.FireCount` 0)
  (bind _returnvalue (`KismetSystemLibrary.K2_SetTimerDelegate` (delegate `Fire`) (`self.FireInterval`) true))
  (set `self.FireTimer` _returnvalue))

(event `Fire`
  (message `/Game/ShootingGame/Blueprints/Player/Enemy/BPI_GetEnemies.GetEnemyChaseBullet` (`GameplayStatics.GetGameMode`) (`SceneComponent.GetSocketTransform` (`self.StaticMesh`) "AttackSocket" "RTS_World"))
  (bind _result (`/Engine/EditorBlueprintResources/StandardMacros.IncrementInt` (`self.FireCount`))
    (:`  `
      (if (>= _result (`self.FireRepeatCount`))
        (`KismetSystemLibrary.K2_ClearAndInvalidateTimerHandle` (`self.FireTimer`))
        (`KismetSystemLibrary.Delay` (`self.FireInterval`))))))

(fn `UserConstructionScript`
  (`parent.UserConstructionScript`))