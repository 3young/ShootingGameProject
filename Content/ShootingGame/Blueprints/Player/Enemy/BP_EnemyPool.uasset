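; BP_EnemyPool is an actor that holds a pool of BP_EnemyFirst enemies for the shooting game.
; On BeginPlay it loops over EnemyChaseTransform and spawns an enemy only while EnemyPool is empty, so just the first transform produces one.
; After adding that enemy to the pool, it hides and disables collision on the pool actor itself, as neither call targets the spawned enemy.
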(event `self.ReceiveBeginPlay`
  (for _array_element (`self.EnemyChaseTransform`)
    (if (<= (`KismetArrayLibrary.Array_Length` (`self.EnemyPool`)) 0)
      (bind _returnvalue (`|SpawnActorFromClass` "/Game/ShootingGame/Blueprints/Player/Enemy/BP_EnemyFirst.BP_EnemyFirst_C" _array_element "AlwaysSpawn" "MultiplyWithRoot" null null))
      (`KismetArrayLibrary.Array_Add` (`self.EnemyPool`) _returnvalue)
      (`self.SetActorHiddenInGame` true)
      (`self.SetActorEnableCollision` false))))

(fn `UserConstructionScript`)