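; BP_EnemyBase is the base enemy for the shooting game, a damageable actor that flies along its forward vector using ProjectileMovement.
; Activation runs only when inactive, restoring full HP, setting velocity from MoveSpeed and enabling the mesh's visibility and query-only collision.
; AnyDamage subtracts HP and deactivates the enemy at zero or below.
; Deactivation hides the mesh, spawns an auto-released pooled SelfExplosion effect and destroys the actor.
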(event `self.OnActivate`
  (bind _staticmesh (`self.StaticMesh`))
  (if (== (`self.IsActivated?`) false)
    (set `self.HP` (`self.MaxHP`))
    (set `MovementComponent.Velocity` (* (`self.GetActorForwardVector`) (`self.MoveSpeed`)) (`self.ProjectileMovement`))
    (`PrimitiveComponent.SetCollisionEnabled` _staticmesh "QueryOnly")
    (`SceneComponent.SetVisibility` _staticmesh true false)
    (set `self.IsActivated?` true)))

(event `self.OnDeactivate`
  (bind _staticmesh (`self.StaticMesh`))
  (`PrimitiveComponent.SetCollisionEnabled` _staticmesh "NoCollision")
  (`SceneComponent.SetVisibility` _staticmesh false false)
  (set `self.IsActivated?` false)
  (`NiagaraFunctionLibrary.SpawnSystemAtLocation` (`self.SelfExplosion`) (`self.K2_GetActorLocation`) (struct) (1.0 1.0 1.0) true true "AutoRelease")
  (`self.K2_DestroyActor`))

(event `self.ReceiveAnyDamage`
  (params (Damage :type "Float (single-precision)") (DamageType :type "DamageType Object Reference") (InstigatedBy :type "Controller Object Reference") (DamageCauser :type "Actor Object Reference"))
  (bind _output_get (set `self.HP` (- (`self.HP`) Damage)))
  (if (<= _output_get 0.0)
    (`self.Deactivate`)))

(fn `UserConstructionScript`
  (`parent.UserConstructionScript`))