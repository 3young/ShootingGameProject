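; First enemy type for the shooting game, which advances, then chases and fires at the player.
; On BeginPlay a timeline pushes it forward by local offsets, then it takes one interpolated turn toward the player and starts an AI move to them.
; After a short delay a looping timer at AttackInterval pulls objects from ACEnemyObjectPool at its own transform to fire.
; Deactivate clears that fire timer.
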(event `self.ReceiveBeginPlay`
  (`Timeline|TL_MoveForward`
    (:`Update`
      (`self.K2_AddActorLocalOffset` (7.0 0.0 0.0)))
    (:`Finished`
      (`self.RotateTowardsPlayer`)
      (`|ExecutionSequence`
        (:`then_0`
          (`self.MoveEnemy`))
        (:`then_1`
          (`KismetSystemLibrary.Delay` 0.2)
          (bind _returnvalue (`KismetSystemLibrary.K2_SetTimerDelegate` (delegate `FireRepeat`) (`self.AttackInterval`) true))
          (set `self.FireTimer` _returnvalue))))))

(event `FireRepeat`
  (`self.Fire`))

(event `Fire`
  (`/Game/ShootingGame/Blueprints/ObjectPool/AC_EnemyObjectPool.GetEnemyObject` (`self.AC_EnemyObjectPool`) (`self.GetTransform`)))

(event `RotateTowardsPlayer`
  (`self.K2_SetActorRotation` (`KismetMathLibrary.RInterpTo` (`self.K2_GetActorRotation`) (`KismetMathLibrary.FindLookAtRotation` (`self.K2_GetActorLocation`) (`self.K2_GetActorLocation` (`GameplayStatics.GetPlayerPawn` 0))) (`GameplayStatics.GetWorldDeltaSeconds`) 20.0)))

(event `MoveEnemy`
  (`|AIMoveTo` (`Controller.K2_GetPawn` (`self.GetController`)) (0.0 0.0 0.0) (`GameplayStatics.GetPlayerPawn` 0) 1.0))

(event `/Game/ShootingGame/Blueprints/ObjectPool/BPI_PoolObject.Deactivate`
  (`KismetSystemLibrary.K2_ClearAndInvalidateTimerHandle` (`self.FireTimer`)))

(fn `UserConstructionScript`
  (`parent.UserConstructionScript`))