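; Player flight pawn for a shooter that moves with Enhanced Input, creates the UI and subtracts damage from HP.
; Four weapons draw bullets from pool components: delay-gated normal (alternating sockets) and main fire, plus timer-driven homing and area fire.
; Only homing sets a looping interval; the area timer has neither time nor looping set.
; Tick teleports past-border positions via OtherSideLocation, whose negated-position vector is left unconnected.
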(event `self.ReceiveBeginPlay`
  (`EnhancedInputSubsystemInterface.AddMappingContext` (pcsubsystem `EnhancedInputLocalPlayerSubsystem` (`GameplayStatics.GetPlayerController` 0)) "/Game/ShootingGame/Input/IMC_PlayerFlight.IMC_PlayerFlight" 0 (struct))
  (set `self.PlayerHp` (`self.PlayerMaxHp`))
  (bind _returnvalue (`|CreateWidget` "/Game/ShootingGame/UI/WBP_UI.WBP_UI_C" (`GameplayStatics.GetPlayerController` 0)))
  (`UserWidget.AddToViewport` _returnvalue 0))

(event `self.ReceiveTick`
  (params (DeltaSeconds :type "Float (single-precision)"))
  (`self.WarpToOtherSide`))

(event `EnhancedInput|/Game/ShootingGame/Input/IA_Move`
  (params (ActionValue :type "Vector2D Structure") (ElapsedSeconds :type "Float (double-precision)") (TriggeredSeconds :type "Float (double-precision)") (InputAction :type "InputAction Object Reference" :default "/Game/ShootingGame/Input/IA_Move.IA_Move"))
  (bind (_returnvalue_x _returnvalue_y) (`KismetMathLibrary.BreakVector2D` (`KismetMathLibrary.Normal2D` ActionValue)))
  (:`Triggered`
    (`self.AddMovementInput` (`KismetMathLibrary.MakeVector` _returnvalue_y _returnvalue_x))))

(event `EnhancedInput|/Game/ShootingGame/Input/IA_Fire`
  (params (ActionValue :type Boolean) (ElapsedSeconds :type "Float (double-precision)") (TriggeredSeconds :type "Float (double-precision)") (InputAction :type "InputAction Object Reference" :default "/Game/ShootingGame/Input/IA_Fire.IA_Fire"))
  (:`Triggered`
    (`self.Fire`)))

(event `Fire`
  (if (`self.IsNormalFireReady`)
    (set `self.IsNormalFireReady` false)
    (bind _firetransform (`self.GetFireTransform`))
    (`/Game/ShootingGame/Blueprints/ObjectPool/AC_ObjectPool.GetObject` (`self.AC_NormalBullet`) _firetransform)
    (`KismetSystemLibrary.Delay` (`self.NormalInterval`))
    (set `self.IsNormalFireReady` true)))

(event `EnhancedInput|/Game/ShootingGame/Input/IA_MainFire`
  (params (ActionValue :type Boolean) (ElapsedSeconds :type "Float (double-precision)") (TriggeredSeconds :type "Float (double-precision)") (InputAction :type "InputAction Object Reference" :default "/Game/ShootingGame/Input/IA_MainFire.IA_MainFire"))
  (:`Triggered`
    (`self.MainFire`)))

(event `MainFire`
  (if (`self.IsMainFireReady`)
    (set `self.IsMainFireReady` false)
    (bind _firetransform (`self.GetMainFireTransform`))
    (`/Game/ShootingGame/Blueprints/ObjectPool/AC_ObjectPool.GetObject` (`self.AC_MainBullet`) _firetransform)
    (`KismetSystemLibrary.Delay` (`self.MainInterval`))
    (set `self.IsMainFireReady` true)))

(event `EnhancedInput|/Game/ShootingGame/Input/IA_FireHoming`
  (params (ActionValue :type Boolean) (ElapsedSeconds :type "Float (double-precision)") (TriggeredSeconds :type "Float (double-precision)") (InputAction :type "InputAction Object Reference" :default "/Game/ShootingGame/Input/IA_FireHoming.IA_FireHoming"))
  (:`Started`
    (`self.FireHoming`)
    (bind _returnvalue (`KismetSystemLibrary.K2_SetTimerDelegate` (delegate `FireHomingRepeat`) (`self.HomingInterval`) true))
    (set `self.HomingTimer` _returnvalue))
  (:`Completed`
    (`KismetSystemLibrary.K2_ClearAndInvalidateTimerHandle` (`self.HomingTimer`))))

(event `FireHomingRepeat`
  (`self.FireHoming`))

(event `FireHoming`
  (`/Game/ShootingGame/Blueprints/ObjectPool/AC_ObjectPool.GetObject` (`self.AC_HomingBullet`) (`self.GetTransform`)))

(event `EnhancedInput|/Game/ShootingGame/Input/IA_FireArea`
  (params (ActionValue :type Boolean) (ElapsedSeconds :type "Float (double-precision)") (TriggeredSeconds :type "Float (double-precision)") (InputAction :type "InputAction Object Reference" :default "/Game/ShootingGame/Input/IA_FireArea.IA_FireArea"))
  (:`Started`
    (`self.FireArea`)
    (bind _returnvalue (`KismetSystemLibrary.K2_SetTimerDelegate` (delegate `FireAreaRepeat`)))
    (set `self.AreaTimer` _returnvalue))
  (:`Completed`
    (`KismetSystemLibrary.K2_ClearAndInvalidateTimerHandle` (`self.AreaTimer`))))

(event `FireAreaRepeat`
  (`self.FireArea`))

(event `FireArea`
  (`/Game/ShootingGame/Blueprints/ObjectPool/AC_ObjectPool.GetObject` (`self.AC_AreaBullet`) (`self.GetTransform`)))

(event `self.ReceiveAnyDamage`
  (params (Damage :type "Float (single-precision)") (DamageType :type "DamageType Object Reference") (InstigatedBy :type "Controller Object Reference") (DamageCauser :type "Actor Object Reference"))
  (set `self.PlayerHp` (- (`self.PlayerHp`) Damage)))

(fn `FireBullet`)

(fn `GetFireTransform`
  (returns (FireTransform :type "Transform Structure"))
  (bind _playerflight (`self.PlayerFlight`))
  (if (`self.FireLocationSelector`)
    (set `self.FireLocationSelector` false)
    (return (`SceneComponent.GetSocketTransform` _playerflight "FireSocket1" "RTS_World"))
    (else
      (set `self.FireLocationSelector` true)
      (return (`SceneComponent.GetSocketTransform` _playerflight "FireSocket2" "RTS_World")))))

(fn `GetMainFireTransform`
  (returns (FireTransform :type "Transform Structure"))
  (return (`SceneComponent.GetSocketTransform` (`self.PlayerFlight`) "FireSocket0" "RTS_World")))

(fn `UserConstructionScript`)

(fn `WarpToOtherSide`
  (locals (BorderY :type Integer :default 3500) (BorderX :type Integer :default 2000))
  (bind (_returnvalue_x _returnvalue_y) (`KismetMathLibrary.BreakVector` (`self.K2_GetActorLocation`)))
  (bind _returnvalue_x_2 (`KismetMathLibrary.BreakVector` (`self.K2_GetActorLocation`)))
  (`|ExecutionSequence`
    (:`then_0`
      (if (> _returnvalue_x_2 (`local.BorderX`))
        (`self.K2_SetActorLocation` (`self.OtherSideLocation`) false true :!label _label)
        (elif (< _returnvalue_x_2 (* (`local.BorderX`) -1))
          (goto _label))))
    (:`then_1`
      (if (> _returnvalue_y (`local.BorderY`))
        (`self.K2_SetActorLocation` (`self.OtherSideLocation`) false true :!label _label_2)
        (elif (< _returnvalue_y (* (`local.BorderY`) -1))
          (goto _label_2))))))