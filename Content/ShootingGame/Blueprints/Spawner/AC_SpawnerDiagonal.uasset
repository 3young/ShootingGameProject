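; Spawner component for the shooting game that releases a wave of enemies one by one in a staggered, diagonal-style line.
; Spawn starts a looping timer that sends the game mode an enemy message with type and transform until SpawnCount is reached.
; Each transform steps further along SpawnArea's right vector by SubSpacing, so time and position offsets combine.
; The BeginPlay validity check only leads to a delay.
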(event `self.ReceiveBeginPlay`
  (`/Engine/EditorBlueprintResources/StandardMacros.IsValid` (`self.SpawnArea`)
    (:`Is Not Valid`
      (`KismetSystemLibrary.Delay` 0.2))))

(event `self.Spawn`
  (bind _returnvalue (`KismetSystemLibrary.K2_SetTimerDelegate` (delegate `SubSpawn`) (`self.SubInterval`) true))
  (set `self.SubSpawnCounter` _returnvalue))

(event `SubSpawn`
  (message `/Game/ShootingGame/Blueprints/Enemy/BPI_GetEnemies.GetEnemy` (`GameplayStatics.GetGameMode`) (`self.SpawnTargetType`) (`self.GetSpawnTransform`))
  (if (== (`self.SpawnIndex`) (`self.SpawnCount`))
    (`KismetSystemLibrary.K2_ClearAndInvalidateTimerHandle` (`self.SubSpawnCounter`))
    (set `self.SpawnIndex` 0)))

(fn `GetSpawnTransform`
  (returns (ReturnValue :type "Transform Structure"))
  (bind _spawnarea (`self.SpawnArea`))
  (`/Engine/EditorBlueprintResources/StandardMacros.IsValid` _spawnarea
    (:`Is Valid`
      (`/Engine/EditorBlueprintResources/StandardMacros.IncrementInt` (`self.SpawnIndex`)
        (:`  `
          (return (`KismetMathLibrary.MakeTransform` (+ (`SceneComponent.K2_GetComponentLocation` _spawnarea) (* (`SceneComponent.GetRightVector` _spawnarea) (`self.SubSpacing`) (- (`self.SpawnIndex`) 1))) (`SceneComponent.K2_GetComponentRotation` (`self.SpawnArea`)))))))
    (:`Is Not Valid`
      (`KismetSystemLibrary.PrintString` "SpawnArea Is Not Valid"))))