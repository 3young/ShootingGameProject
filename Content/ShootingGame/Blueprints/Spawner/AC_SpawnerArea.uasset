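; Actor component that asks the game mode for an enemy of a set target type within a spawn area.
; Spawn sends that type and a generated transform through GetEnemyMessage on the game mode.
; The transform picks random X and Y within the area component's bounds, keeping its Z, rotation and scale.
; BeginPlay only delays briefly when the area reference is invalid, with no follow-up action.
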(event `self.ReceiveBeginPlay`
  (`/Engine/EditorBlueprintResources/StandardMacros.IsValid` (`self.SpawnArea`)
    (:`Is Not Valid`
      (`KismetSystemLibrary.Delay` 0.2))))

(event `self.Spawn`
  (message `/Game/ShootingGame/Blueprints/Enemy/BPI_GetEnemies.GetEnemy` (`GameplayStatics.GetGameMode`) (`self.SpawnTargetType`) (`self.GetSpawnTransform`)))

(fn `GetSpawnTransform`
  (returns (ReturnValue :type "Transform Structure"))
  (bind _spawnarea (`self.SpawnArea`))
  (bind (_origin _boxextent) (`KismetSystemLibrary.GetComponentBounds` _spawnarea))
  (bind _returnvalue (`SceneComponent.K2_GetComponentToWorld` _spawnarea))
  (bind (_min _max) (`self.GetBoxMinMax` (.x _origin) (.x _boxextent)))
  (bind (_min_2 _max_2) (`self.GetBoxMinMax` (.y _origin) (.y _boxextent)))
  (return (`KismetMathLibrary.MakeTransform` (`KismetMathLibrary.MakeVector` (`KismetMathLibrary.RandomFloatInRange` _min _max) (`KismetMathLibrary.RandomFloatInRange` _min_2 _max_2) (.z (.location _returnvalue))) (.rotation _returnvalue) (.scale _returnvalue))))