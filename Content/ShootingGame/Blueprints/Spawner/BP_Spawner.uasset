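; BP_Spawner is an enemy spawner for the shooting game that runs one scripted sequence of chase, wave and boss enemies.
; BeginPlay sets a short timer, apparently to trigger SpawnEnemies, which spawns chase enemies, then a wave enemy and a boss after delays, and finally clears a timer handle.
; The construction script assigns spawn areas to three spawner components, but SpawnEnemies spawns actors directly at those areas' transforms.
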(event `self.ReceiveBeginPlay`
  (`KismetSystemLibrary.K2_SetTimerDelegate` (`|CreateDelegate` (`self.SpawnerMass`) :!event `Spawn`) 2.0))

(event `SpawnEnemies`
  (for _ (range 2)
    (`|SpawnActorFromClass` "/Game/ShootingGame/Blueprints/Enemy/BP_EnemyChase.BP_EnemyChase_C" (`SceneComponent.K2_GetComponentToWorld` (`self.SpawnAreaMass`)) "AlwaysSpawn" "MultiplyWithRoot" null null))
  (`KismetSystemLibrary.Delay` 5.0)
  (`|SpawnActorFromClass` "/Game/ShootingGame/Blueprints/Enemy/BP_EnemyWave.BP_EnemyWave_C" (`SceneComponent.K2_GetComponentToWorld` (`self.SpawnAreaDiagonal`)) "AlwaysSpawn" "MultiplyWithRoot" null null)
  (`KismetSystemLibrary.Delay` 0.2)
  (`|SpawnActorFromClass` "/Game/ShootingGame/Blueprints/Enemy/BP_EnemyBoss.BP_EnemyBoss_C" (`SceneComponent.K2_GetComponentToWorld` (`self.SpawnAreaArea`)) "AlwaysSpawn" "MultiplyWithRoot" null null)
  (`KismetSystemLibrary.K2_ClearAndInvalidateTimerHandle` (`self.NewVar`)))

(fn `UserConstructionScript`
  (set `/Game/ShootingGame/Blueprints/Spawner/AC_SpawnerBase.SpawnArea` (`self.SpawnAreaMass`) (`self.SpawnerMass`))
  (set `/Game/ShootingGame/Blueprints/Spawner/AC_SpawnerBase.SpawnArea` (`self.SpawnAreaDiagonal`) (`self.SpawnerDiagonal`))
  (set `/Game/ShootingGame/Blueprints/Spawner/AC_SpawnerBase.SpawnArea` (`self.SpawnAreaArea`) (`self.SpawnerArea`)))