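; AC_SpawnerMass is a spawner component that spawns a group of enemies in a ring around its spawn transform.
; On Spawn, it spaces MassCount points evenly around a circle of the given Radius in the XY plane, keeping the center's height, rotation and scale.
; For each point it sends a GetEnemy message with SpawnTargetType to the game mode, leaving the provision of enemies to it.
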(event `self.Spawn`
  (bind _radius (`self.Radius`))
  (bind (_spawntransform_location _spawntransform_rotation _spawntransform_scale) (`KismetMathLibrary.BreakTransform` (`self.SpawnTransform`)))
  (bind _spawntransform (`self.SpawnTransform`))
  (set `self.SpawnTransform` (`self.GetSpawnTransform`))
  (for _index (range (`self.MassCount`))
    (bind _output_get (set `self.Angle` (/ (* _index 360.0) (`self.MassCount`))))
    (bind _returnvalue (`KismetMathLibrary.DegreesToRadians` _output_get))
    (message `/Game/ShootingGame/Blueprints/Enemy/BPI_GetEnemies.GetEnemy` (`GameplayStatics.GetGameMode`) (`self.SpawnTargetType`) (`KismetMathLibrary.MakeTransform` (`KismetMathLibrary.MakeVector` (+ (* (`KismetMathLibrary.Cos` _returnvalue) _radius) (.x (.location _spawntransform))) (+ (* _radius (`KismetMathLibrary.Sin` _returnvalue)) (.y (.location _spawntransform))) (.z (.location _spawntransform))) _spawntransform_rotation _spawntransform_scale))))