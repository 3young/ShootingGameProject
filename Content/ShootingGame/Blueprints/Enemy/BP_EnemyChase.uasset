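; BP_EnemyChase is a shooting-game enemy that pursues the player pawn and fires at intervals once activated.
; Each Tick it eases its location and rotation toward the player with interpolation, using a fixed delta time for the turn.
; A Delay inside Tick paces Fire, which spawns a BP_EnemyChaseBullet at the mesh's AttackSocket and activates it.
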(event `self.OnActivate`
  (`parent.OnActivate`)
  (set `self.CanMove` true))

(event `self.ReceiveTick`
  (params (DeltaSeconds :type "Float (single-precision)"))
  (bind _returnvalue (`GameplayStatics.GetPlayerPawn` 0))
  (if (`self.CanMove`)
    (`/Engine/EditorBlueprintResources/StandardMacros.IsValid` _returnvalue
      (:`Is Valid`
        (`self.K2_SetActorLocation` (`KismetMathLibrary.VInterpTo` (`self.K2_GetActorLocation`) (`self.K2_GetActorLocation` _returnvalue) (`GameplayStatics.GetWorldDeltaSeconds`) 0.1))
        (`self.RotateTowardsPlayer`)
        (`KismetSystemLibrary.Delay` (`self.FireInterval`))
        (`self.Fire`)))))

(event `Fire`
  (bind _returnvalue (`|SpawnActorFromClass` "/Game/ShootingGame/Blueprints/Enemy/BP_EnemyChaseBullet.BP_EnemyChaseBullet_C" (`SceneComponent.GetSocketTransform` (`self.StaticMesh`) "AttackSocket" "RTS_World") "AlwaysSpawn" "MultiplyWithRoot" null null))
  (bind _asbp_enemy_chase_bullet (cast `/Game/ShootingGame/Blueprints/Enemy/BP_EnemyChaseBullet` _returnvalue))
  (`self.OnActivate` _asbp_enemy_chase_bullet))

(event `RotateTowardsPlayer`
  (set `self.LookAtLocation` (`self.K2_GetActorLocation` (`GameplayStatics.GetPlayerPawn` 0)))
  (`self.K2_SetActorRotation` (`KismetMathLibrary.RInterpTo` (`self.K2_GetActorRotation`) (`KismetMathLibrary.FindLookAtRotation` (`self.K2_GetActorLocation`) (`self.LookAtLocation`)) 2.0 0.1)))

(fn `UserConstructionScript`
  (`parent.UserConstructionScript`))