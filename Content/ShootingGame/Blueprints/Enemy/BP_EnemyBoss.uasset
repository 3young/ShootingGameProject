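; BP_EnemyBoss is the boss enemy of the shooting game, firing bullets at a regular interval once activated.
; OnActivate runs the parent's activation, then starts a looping timer driven by FireInterval.
; Each timer tick spawns a BP_EnemyBossBullet at the mesh's AttackSocket transform, ignoring collisions, and calls OnActivate on it.
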(event `self.OnActivate`
  (`parent.OnActivate`)
  (`self.FireProcess`))

(event `FireProcess`
  (`KismetSystemLibrary.K2_SetTimerDelegate` (delegate `Fire`) (`self.FireInterval`) true))

(event `Fire`
  (bind _returnvalue (`|SpawnActorFromClass` "/Game/ShootingGame/Blueprints/Enemy/BP_EnemyBossBullet.BP_EnemyBossBullet_C" (`SceneComponent.GetSocketTransform` (`self.StaticMesh`) "AttackSocket" "RTS_World") "AlwaysSpawn" "MultiplyWithRoot" null null))
  (bind _asbp_enemy_boss_bullet (cast `/Game/ShootingGame/Blueprints/Enemy/BP_EnemyBossBullet` _returnvalue))
  (`self.OnActivate` _asbp_enemy_boss_bullet))

(fn `UserConstructionScript`
  (`parent.UserConstructionScript`))