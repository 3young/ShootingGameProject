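; BP_EnemyWaveBullet is an enemy projectile that flies along its mesh's forward vector and damages Player-tagged actors on overlap.
; OnActivate sets velocity, shows the mesh, enables query collision and starts a lifetime timer, suggesting reuse through pooling.
; OnDeactivate, also called after a hit, only zeroes velocity and sets an initialization flag.
; Its explosion effect, mesh hiding and collision disabling are disconnected and never run.
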(event `self.OnActivate`
  (bind _staticmesh (`self.StaticMesh`))
  (set `MovementComponent.Velocity` (* (`SceneComponent.GetForwardVector` (`self.StaticMesh`)) (`self.MoveSpeed`)) (`self.ProjectileMovement`))
  (`PrimitiveComponent.SetCollisionEnabled` _staticmesh "QueryOnly")
  (`SceneComponent.SetVisibility` _staticmesh true false)
  (`KismetSystemLibrary.K2_SetTimerDelegate` (`|CreateDelegate` :!event `Deactivate`) (`self.LifeTime`)))

(event `self.OnDeactivate`
  (set `MovementComponent.Velocity` (0.0 0.0 0.0) (`self.ProjectileMovement`))
  (if (not (`self.IsInitialized`))
    (set `self.IsInitialized` true)))

(event `self.ReceiveActorBeginOverlap`
  (params (OtherActor :type "Actor Object Reference"))
  (if (`self.ActorHasTag` OtherActor "Player")
    (`GameplayStatics.ApplyDamage` OtherActor (`self.BaseDamage`))
    (`self.OnDeactivate`)))

(fn `UserConstructionScript`)