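; Enemy bullet for the shooting game that fires toward the player's position and damages actors tagged Player.
; OnActivate sets the velocity once, without continuous homing, shows the mesh, enables query collision and starts a lifetime timer.
; Overlapping the player spawns an explosion effect, applies damage and calls OnDeactivate.
; OnDeactivate hides the bullet and disables collision instead of destroying it, optionally spawning an immediately deactivated explosion effect.
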(event `self.OnActivate`
  (bind _returnvalue (`GameplayStatics.GetPlayerPawn` 0))
  (bind _staticmesh (`self.StaticMesh`))
  (`/Engine/EditorBlueprintResources/StandardMacros.IsValid` _returnvalue
    (:`Is Valid`
      (`ActorComponent.SetActive` (`self.ProjectileMovement`) true false)
      (set `MovementComponent.Velocity` (* (`KismetMathLibrary.Normal` (- (`self.K2_GetActorLocation` _returnvalue) (`self.K2_GetActorLocation`))) (`self.MoveSpeed`)) (`self.ProjectileMovement`))
      (`PrimitiveComponent.SetCollisionEnabled` _staticmesh "QueryOnly")
      (`SceneComponent.SetVisibility` _staticmesh true false)
      (`KismetSystemLibrary.K2_SetTimerDelegate` (`|CreateDelegate` :!event `Deactivate`) (`self.LifeTime`)))))

(event `self.OnDeactivate`
  (bind _staticmesh (`self.StaticMesh`))
  (`SceneComponent.SetVisibility` _staticmesh false false)
  (`PrimitiveComponent.SetCollisionEnabled` _staticmesh "NoCollision")
  (if (`self.bShouldExplosion`)
    (bind _returnvalue (`NiagaraFunctionLibrary.SpawnSystemAtLocation` (`self.SelfExplosion`) (`self.K2_GetActorLocation`) (struct) (1.0 1.0 1.0) true true "AutoRelease"))
    (`ActorComponent.Deactivate` _returnvalue)
    (set `self.bShouldExplosion` true)))

(event `self.ReceiveActorBeginOverlap`
  (params (OtherActor :type "Actor Object Reference"))
  (if (`self.ActorHasTag` OtherActor "Player")
    (`NiagaraFunctionLibrary.SpawnSystemAtLocation` (`self.SelfExplosion`) (`self.K2_GetActorLocation`) (struct) (1.0 1.0 1.0) true true "AutoRelease")
    (`GameplayStatics.ApplyDamage` OtherActor (`self.BaseDamage`))
    (`self.OnDeactivate`)))

(fn `UserConstructionScript`)