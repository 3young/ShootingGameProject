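; Base enemy for the shooting game, toggled on and off through activate and deactivate events rather than spawned or destroyed.
; Activation restores HP, launches it forward and enables tick, visibility and query collision; deactivation reverses these states and spawns a pooled explosion.
; Incoming damage reduces HP, prints debug text and, at zero, awards points through the GameState and deactivates.
; Overlapping the player runs a looping timer applying tick-scaled damage until overlap ends.
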(event `self.OnActivate`
  (bind _staticmesh (`self.StaticMesh`))
  (if (== (`self.IsActivated?`) false)
    (`self.SetActorTickEnabled` true)
    (set `self.HP` (`self.MaxHP`))
    (set `MovementComponent.Velocity` (* (`self.GetActorForwardVector`) (`self.MoveSpeed`)) (`self.ProjectileMovement`))
    (`PrimitiveComponent.SetCollisionEnabled` _staticmesh "QueryOnly")
    (`SceneComponent.SetVisibility` _staticmesh true false)
    (set `self.IsActivated?` true)))

(event `self.OnDeactivate`
  (bind _staticmesh (`self.StaticMesh`))
  (if (== (`self.IsActivated?`) true)
    (`PrimitiveComponent.SetCollisionEnabled` _staticmesh "NoCollision")
    (`SceneComponent.SetVisibility` _staticmesh false false)
    (set `self.IsActivated?` false)
    (`self.SetActorTickEnabled` false)
    (`NiagaraFunctionLibrary.SpawnSystemAtLocation` (`self.SelfExplosion`) (`self.K2_GetActorLocation`) (struct) (1.0 1.0 1.0) true true "AutoRelease")))

(event `self.ReceiveAnyDamage`
  (params (Damage :type "Float (single-precision)") (DamageType :type "DamageType Object Reference") (InstigatedBy :type "Controller Object Reference") (DamageCauser :type "Actor Object Reference"))
  (bind _output_get (set `self.HP` (- (`self.HP`) Damage)))
  (if (<= _output_get 0.0)
    (message `/Game/ShootingGame/Blueprints/Frameworks/BPI_Score.AddScore` (`GameplayStatics.GetGameState`) (`self.Point`))
    (`self.Deactivate`))
  (`KismetSystemLibrary.PrintString` (`KismetStringLibrary.BuildString_Double` (`KismetStringLibrary.BuildString_Double` (`KismetStringLibrary.BuildString_Double` "HP:" "[" (`self.HP`) "/") "" (`self.MaxHP`) "]") "" (`KismetSystemLibrary.GetGameTimeInSeconds`))))

(event `self.ReceiveActorBeginOverlap`
  (params (OtherActor :type "Actor Object Reference"))
  (if (and (`self.ActorHasTag` OtherActor "Player") (not (`KismetSystemLibrary.K2_IsValidTimerHandle` (`self.DamageTimer`))))
    (bind _returnvalue (`KismetSystemLibrary.K2_SetTimerDelegate` (delegate `PlayerAttack`) (`self.DamageTick`) true))
    (set `self.DamageTimer` _returnvalue)))

(event `PlayerAttack`
  (`GameplayStatics.ApplyDamage` (stale `self.ReceiveActorBeginOverlap` OtherActor) (* (`self.BaseDamage`) (`self.DamageTick`))))

(event `self.ReceiveActorEndOverlap`
  (params (OtherActor :type "Actor Object Reference"))
  (if (`self.ActorHasTag` OtherActor "Player")
    (`KismetSystemLibrary.K2_ClearAndInvalidateTimerHandle` (`self.DamageTimer`))))

(fn `UserConstructionScript`
  (`parent.UserConstructionScript`))