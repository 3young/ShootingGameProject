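; BP_EnemyWave is a shooting-game enemy that sways sideways while firing bullets from two sockets.
; On activation it plays the TL_Wave timeline, offsetting its mesh's relative location along the left vector by WaveAlpha times Width.
; It also starts two looping timers sharing FireInterval, each spawning a BP_EnemyWaveBullet at its own attack socket and activating it.
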(event `self.OnActivate`
  (`parent.OnActivate`)
  (`|ExecutionSequence`
    (:`then_0`
      (bind (_direction _wavealpha) (`Timeline|TL_Wave` :!via `PlayFromStart`)
        (:`Update`
          (`SceneComponent.K2_SetRelativeLocation` (`self.StaticMesh`) (* _wavealpha (`self.Width`) (`KismetMathLibrary.Vector_Left`)) false false))))
    (:`then_1`
      (`self.FireProcess`))))

(event `FireLeft`
  (bind _returnvalue (`|SpawnActorFromClass` "/Game/ShootingGame/Blueprints/Enemy/BP_EnemyWaveBullet.BP_EnemyWaveBullet_C" (`SceneComponent.GetSocketTransform` (`self.StaticMesh`) "AttackSocket2" "RTS_World") "AlwaysSpawn" "MultiplyWithRoot" null null))
  (bind _asbp_enemy_wave_bullet (cast `/Game/ShootingGame/Blueprints/Enemy/BP_EnemyWaveBullet` _returnvalue))
  (`self.OnActivate` _asbp_enemy_wave_bullet))

(event `FireProcess`
  (`|ExecutionSequence`
    (:`then_0`
      (`KismetSystemLibrary.K2_SetTimerDelegate` (delegate `FireLeft`) (`self.FireInterval`) true))
    (:`then_1`
      (`KismetSystemLibrary.K2_SetTimerDelegate` (delegate `FireRight`) (`self.FireInterval`) true))))

(event `FireRight`
  (bind _returnvalue (`|SpawnActorFromClass` "/Game/ShootingGame/Blueprints/Enemy/BP_EnemyWaveBullet.BP_EnemyWaveBullet_C" (`SceneComponent.GetSocketTransform` (`self.StaticMesh`) "AttackSocket1" "RTS_World") "AlwaysSpawn" "MultiplyWithRoot" null null))
  (bind _asbp_enemy_wave_bullet (cast `/Game/ShootingGame/Blueprints/Enemy/BP_EnemyWaveBullet` _returnvalue))
  (`self.OnActivate` _asbp_enemy_wave_bullet))

(fn `UserConstructionScript`
  (`parent.UserConstructionScript`))